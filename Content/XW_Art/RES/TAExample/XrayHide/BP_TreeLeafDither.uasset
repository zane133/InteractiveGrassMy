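; Fades out foliage, likely trees, that blocks the camera's view of the player character.
; A looping timer sphere-traces on the Visibility channel from above the character to the camera, with the start offset by the check radius.
; A hit actor's BPC_TreeFadeComponent starts fading out, and the previous one fades back in when replaced or when nothing is hit.
; An older material-parameter-collection and dynamic-material fade remains disconnected.
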(event `self.ReceiveBeginPlay`
  ; 初始化
  (`KismetSystemLibrary.K2_SetTimerDelegate` (delegate `DoTrace`) 0.1 true true)
  (set `self.CurrentEffectAmount` 0.0))

(event `DoTrace`
  (bind _lasthitfadecomponent (`self.LastHitFadeComponent`))
  (bind _returnvalue (`PlayerCameraManager.GetCameraLocation` (`GameplayStatics.GetPlayerCameraManager` 0)))
  (bind _returnvalue_2 (+ (`SceneComponent.K2_GetComponentLocation` (`Character.Mesh` (`GameplayStatics.GetPlayerCharacter` 0))) (0.0 0.0 100.0)))
  (`|ExecutionSequence`
    (:`then_0`
      ; 角色->相机  射线
      (bind (_outhit _returnvalue_3) (`KismetSystemLibrary.SphereTraceSingle` :`Start` (+ (* (`KismetMathLibrary.Normal` (- _returnvalue _returnvalue_2)) (`self.CheckRadius`)) _returnvalue_2) :`End` _returnvalue :`Radius` (`self.CheckRadius`) :`TraceChannel` "TraceTypeQuery1" :`DrawDebugType` (`self.Draw Debug Type`) :`DrawTime` 0.1))
      (if _returnvalue_3
        (bind _returnvalue_4 (`self.GetComponentByClass` (`.HitActor` (`GameplayStatics.BreakHitResult` _outhit)) "/Game/XW_Art/RES/TAExample/XrayHide/BPC_TreeFadeComponent.BPC_TreeFadeComponent_C"))
        (`/Engine/EditorBlueprintResources/StandardMacros.IsValid` _returnvalue_4
          (:`Is Valid`
            (if (!= _returnvalue_4 (`self.LastHitFadeComponent`))
              (`/Engine/EditorBlueprintResources/StandardMacros.IsValid` _lasthitfadecomponent
                (:`Is Valid`
                  (`/Game/XW_Art/RES/TAExample/XrayHide/BPC_TreeFadeComponent.StartFadeIn` _lasthitfadecomponent))
                (:`Is Not Valid`
                  _))
              (set `self.LastHitFadeComponent` _returnvalue_4)
              (`/Game/XW_Art/RES/TAExample/XrayHide/BPC_TreeFadeComponent.StartFadeOut` _returnvalue_4))))
        (else
          (`/Engine/EditorBlueprintResources/StandardMacros.IsValid` (`self.LastHitFadeComponent`)
            (:`Is Valid`
              (`/Game/XW_Art/RES/TAExample/XrayHide/BPC_TreeFadeComponent.StartFadeIn` (`self.LastHitFadeComponent`))
              (set `self.LastHitFadeComponent` null))))))))

(event `self.ReceiveTick`
  (params (DeltaSeconds :type "Float (single-precision)"))
  ; 插值动画
)

(fn `UserConstructionScript`)