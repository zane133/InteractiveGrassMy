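; Actor component that fades a tree's static mesh out and back in through material parameters, as part of an X-ray hide example.
; On BeginPlay it replaces each material on the owner's static mesh component with a dynamic instance.
; StartFadeOut and StartFadeIn set the target effect amount and enable Tick.
; Tick interpolates toward that target, writes EffectAmount and FadeHeightOffset to every instance, and disables itself when close.
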(event `self.ReceiveBeginPlay`
  (bind _returnvalue (`Actor.GetComponentByClass` (`self.GetOwner`) "/Script/Engine.StaticMeshComponent"))
  (for _index (range (+ (- (`PrimitiveComponent.GetNumMaterials` _returnvalue) 1) 1))
    (bind _returnvalue_2 (`KismetMaterialLibrary.CreateDynamicMaterialInstance` (`PrimitiveComponent.GetMaterial` _returnvalue _index)))
    (`KismetArrayLibrary.Array_Add` (`self.DynamicMaterials`) _returnvalue_2)
    (`PrimitiveComponent.SetMaterial` _returnvalue _index _returnvalue_2)))

(event `self.ReceiveTick`
  (params (DeltaSeconds :type "Float (single-precision)"))
  ; 动画
  (set `self.CurrentEffectAmount` (`KismetMathLibrary.FInterpTo` (`self.CurrentEffectAmount`) (`self.TargetEffectAmount`) DeltaSeconds (`self.FadeSpeed`)))
  (for _array_element (`self.DynamicMaterials`)
    (`MaterialInstanceDynamic.SetScalarParameterValue` _array_element "EffectAmount" (`self.CurrentEffectAmount`))
    (`MaterialInstanceDynamic.SetScalarParameterValue` _array_element "FadeHeightOffset" (`self.FadeHeightOffset`))
    (if (`KismetMathLibrary.NearlyEqual_FloatFloat` (`self.CurrentEffectAmount`) (`self.TargetEffectAmount`) 0.01)
      (`self.SetComponentTickEnabled` false))))

(event `StartFadeOut`
  (set `self.TargetEffectAmount` 1.0)
  (`self.SetComponentTickEnabled` true))

(event `StartFadeIn`
  (set `self.TargetEffectAmount` 0.0)
  (`self.SetComponentTickEnabled` true))