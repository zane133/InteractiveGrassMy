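; Grass interaction actor that records the player's trampling in render targets around the character and publishes player position, grass height and bend angle to MPC_Grass_Interaction2.
; Each tick a force material draws a damped spring response, with no brush while falling and optional speed-scaled radius so standing still leaves grass unpressed.
; An offset material then shifts the field by player movement as the actor follows.
; Both passes ping-pong between two targets, cleared on EndPlay.
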(event `self.ReceiveBeginPlay`
  (set `self.LastPos` (`self.K2_GetActorLocation` (`GameplayStatics.GetPlayerCharacter` 0)))
  (`self.CreateMID`)
  (set `self.RT_Temp` "/Game/XW_Art/RES/TAExample/GrassInteraction/RT/RT_Temp.RT_Temp")
  (set `self.RT0` "/Game/XW_Art/RES/TAExample/GrassInteraction/RT/RT_0.RT_0")
  (set `self.RT1` "/Game/XW_Art/RES/TAExample/GrassInteraction/RT/RT_1.RT_1"))

(event `self.ReceiveTick`
  (params (DeltaSeconds :type "Float (single-precision)"))
  (`KismetMaterialLibrary.SetVectorParameterValue` "/Game/XW_Art/RES/TAExample/GrassInteraction/Blueprint/MPC_Grass_Interaction2.MPC_Grass_Interaction2" "PlayerPos" (`KismetMathLibrary.Conv_VectorToLinearColor` (`self.K2_GetActorLocation` (`GameplayStatics.GetPlayerCharacter` 0))))
  (`self.Force1`)
  (`self.Offset2`)
  (`self.UpdataParam`))

(event `UpdataParam`
  (`KismetMaterialLibrary.SetScalarParameterValue` "/Game/XW_Art/RES/TAExample/GrassInteraction/Blueprint/MPC_Grass_Interaction2.MPC_Grass_Interaction2" "GrassHeight" (`self.GrassHeight`))
  (`KismetMaterialLibrary.SetScalarParameterValue` "/Game/XW_Art/RES/TAExample/GrassInteraction/Blueprint/MPC_Grass_Interaction2.MPC_Grass_Interaction2" "BendAnlge" (`self.BendAngle`)))

(event `self.ReceiveEndPlay`
  (params (EndPlayReason :type "EEndPlayReason Enum" :default "Destroyed"))
  (`self.ClearRT`))

(fn `ClearRT`
  (`KismetRenderingLibrary.ClearRenderTarget2D` (`self.RT_Temp`))
  (`KismetRenderingLibrary.ClearRenderTarget2D` (`self.RT0`))
  (`KismetRenderingLibrary.ClearRenderTarget2D` (`self.RT1`)))

(fn `CreateMID`
  (bind _returnvalue (`KismetMaterialLibrary.CreateDynamicMaterialInstance` "/Game/XW_Art/RES/TAExample/GrassInteraction/Mat/M_Force_Grass.M_Force_Grass" "None"))
  (`BlueprintMapLibrary.Map_Add` (`self.DIMMap`) "Force" _returnvalue)
  (bind _returnvalue_2 (`KismetMaterialLibrary.CreateDynamicMaterialInstance` "/Game/XW_Art/RES/TAExample/GrassInteraction/Mat/M_Offset_Grass.M_Offset_Grass" "None"))
  (`BlueprintMapLibrary.Map_Add` (`self.DIMMap`) "Offset" _returnvalue_2))

(fn `Force1`
  (locals (NewLocalVar :type "Vector Structure"))
  (bind _centeruv (`self.CenterUV`))
  (bind _value (`BlueprintMapLibrary.Map_Find` (`self.DIMMap`) "Force"))
  ; Force
  (`/Engine/EditorBlueprintResources/StandardMacros.IsValid` _value
    (:`Is Valid`
      (set `self.CurPosUV` _centeruv)
      (`MaterialInstanceDynamic.SetVectorParameterValue` _value "_InputPos" (`KismetMathLibrary.Conv_VectorToLinearColor` _centeruv))
      (`MaterialInstanceDynamic.SetVectorParameterValue` _value "_ForceVec" (`KismetMathLibrary.Conv_VectorToLinearColor` (`KismetMathLibrary.ClampVectorSize` (- (`self.CurPosUV`) (`self.LastPosUV`)) 0.0 (`self.ForceClampMax `))))
      (set `self.LastPosUV` (`self.CurPosUV`))
      (`MaterialInstanceDynamic.SetTextureParameterValue` _value "_Tex0" (`self.RT0`))
      (`MaterialInstanceDynamic.SetScalarParameterValue` _value "_Radius" (* (`KismetMathLibrary.SelectFloat` 1.0 (* (`KismetMathLibrary.VSizeXY` (`self.GetVelocity` (`GameplayStatics.GetPlayerCharacter` 0))) 0.002) (`self.停下压草`)) (`KismetMathLibrary.SelectFloat` 0.0 (* (`self.Radius`) 0.01) (`NavMovementInterface.IsFalling` (`Character.CharacterMovement` (`GameplayStatics.GetPlayerCharacter` 0))))))
      (`MaterialInstanceDynamic.SetScalarParameterValue` _value "_Damping" (`self.Damping`))
      (`MaterialInstanceDynamic.SetVectorParameterValue` _value "_PlayerSpeed" (`KismetMathLibrary.Conv_VectorToLinearColor` (`self.GetVelocity` (`GameplayStatics.GetPlayerCharacter` 0))))
      (`MaterialInstanceDynamic.SetScalarParameterValue` _value "_SpringK" (`self.SprintK`))
      (`KismetRenderingLibrary.DrawMaterialToRenderTarget` (`self.RT1`) _value)
      (`self.SwapRT0RT1`))))

(fn `Offset2`
  (bind _value (`BlueprintMapLibrary.Map_Find` (`self.DIMMap`) "Offset"))
  (bind _returnvalue_x (`KismetMathLibrary.BreakVector` (`SceneComponent.K2_GetComponentScale` (`self.TraceMesh`))))
  (bind _returnvalue (* _returnvalue_x 100.0))
  (set `self.PlayerVelocity` (`self.GetVelocity` (`GameplayStatics.GetPlayerCharacter` 0)))
  (set `self.TexelSize` (/ _returnvalue (`self.N`)))
  (`/Engine/EditorBlueprintResources/StandardMacros.IsValid` _value
    (:`Is Valid`
      (`MaterialInstanceDynamic.SetTextureParameterValue` _value "RT" (`self.RT0`))
      (`MaterialInstanceDynamic.SetScalarParameterValue` _value "Size" _returnvalue)
      (`MaterialInstanceDynamic.SetVectorParameterValue` _value "PosAndLastPos" (make `LinearColor` (.x (.location (`self.GetTransform` (`GameplayStatics.GetPlayerCharacter` 0)))) (.y (.location (`self.GetTransform` (`GameplayStatics.GetPlayerCharacter` 0)))) (.x (`self.LastPos`)) (.y (`self.LastPos`))))
      (`KismetRenderingLibrary.DrawMaterialToRenderTarget` (`self.RT1`) _value)
      (bind _output_get (set `self.LastPos` (.location (`self.GetTransform` (`GameplayStatics.GetPlayerCharacter` 0)))))
      (`SceneComponent.K2_SetWorldLocation` (`self.DefaultSceneRoot`) (- _output_get (0.0 0.0 80.0)) false false)
      (`self.SwapRT0RT1`))))

(fn `SwapRT0RT1`
  (set `self.RT_Temp` (`self.RT0`))
  (set `self.RT0` (`self.RT1`))
  (set `self.RT1` (`self.RT_Temp`)))

(fn `UpdateParam`)

(fn `UserConstructionScript`)