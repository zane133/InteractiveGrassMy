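; BP_PCG_FenceGrammar is a spline actor in a PCG example folder, named for grammar-based fence generation, with a utility to drape its spline over the ground.
; SnapSplineToGround traces vertically on the Visibility channel, from above to far below each spline point, and moves the point to any hit location.
; The construction script is empty, and the Blueprint graphs contain no fence generation logic.
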(event Custom|SnapSplineToGround
  (for _index (range 0 (- (Spline|GetNumberOfSplinePoints (Variables|Default|GetSpline)) 1))
    (bind (_outhit _returnvalue) (Collision|LineTraceByChannel (+ (Spline|GetLocationatSplinePoint (Variables|Default|GetSpline) _index "World") "0.000000,0.000000,1000.000000") (- (Spline|GetLocationatSplinePoint (Variables|Default|GetSpline) _index "World") "0.000000,0.000000,10000.000000") "TraceTypeQuery1" false 0 "None"))
    (if _returnvalue
      (Spline|SetLocationatSplinePoint (Variables|Default|GetSpline) _index (.Location (Collision|BreakHitResult _outhit)) "World" true))))

(event EventBeginPlay)

(event Collision|EventActorBeginOverlap
  (params (OtherActor :type Actor%20Object%20Reference)))

(event EventTick
  (params (DeltaSeconds :type Float%20%28single-precision%29)))

(fn ConstructionScript)